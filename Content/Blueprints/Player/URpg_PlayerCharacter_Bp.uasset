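; Player character Blueprint for URpg that captures movement input, apparently for animation use.
; After the parent's post-login events run, it casts its controller to URpg_PlayerController and binds to the strafe and forward/back move dispatchers.
; The bound events store the incoming axis values in MoveX and MoveY, ignoring Direction, and a debug print reports the binding.
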(event `self.RunPostLoginEvents`
  (`parent.RunPostLoginEvents`)
  (`self.BindXY`))

(event `BindXY`
  (bind _asurpg_player_controller (cast `URpg_PlayerController` (`self.GetController`)))
  (add `URpg_PlayerController.Move_Strafe` _asurpg_player_controller (delegate `Move_Strafe_Event`))
  (add `URpg_PlayerController.Move_ForwardBack` _asurpg_player_controller (delegate `Move_ForwardBack_Event`))
  (`KismetSystemLibrary.PrintString` null "Binding Anims"))

(event `Move_Strafe_Event`
  (params (Direction :type "Vector Structure (by ref)") (value :type "Float (double-precision) (by ref)"))
  (set `self.MoveX` value))

(event `Move_ForwardBack_Event`
  (params (Direction :type "Vector Structure (by ref)") (value :type "Float (double-precision) (by ref)"))
  (set `self.MoveY` value))

(fn `UserConstructionScript`)