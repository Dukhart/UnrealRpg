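; RPG player controller Blueprint that lets the player kill or respawn themselves through a KillSwitch input.
; Holding the input runs a looping timer that counts hold time; on release, a living player dies if the threshold is met, while a dead one respawns regardless.
; Both actions go through the game mode behind gates that close after firing and reopen via OpenKillGate, with debug prints throughout.
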(event `Key|K`
  (params (Key :type "Key Structure" :default "AnyKey")))

(event `InputAction|KillSwitch`
  (params (Key :type "Key Structure" :default "AnyKey"))
  (:`Pressed`
    (bind _returnvalue (`KismetSystemLibrary.K2_SetTimerDelegate` (delegate `KillTimer`) 0.1 true)))
  (:`Released`
    (`KismetSystemLibrary.K2_ClearTimerHandle` null _returnvalue)
    (if (`self.bIsAlive`)
      (if (>= (`self.KillHoldTimer`) (`self.KillHoldTime`))
        (set `self.KillHoldTimer` 0.0)
        (`/Engine/EditorBlueprintResources/StandardMacros.Gate` false :!label _label
          (:`Exit`
            (`KismetSystemLibrary.PrintString` null "Kill")
            (`self.CloseKillGate`)
            (bind _asurpg_game_mode (cast `URpg_GameMode` (`GameplayStatics.GetGameMode` null)))
            (`URpg_GameMode.KillPlayer` _asurpg_game_mode self)))
        (else
          (set `self.KillHoldTimer` 0.0)))
      (else
        (set `self.KillHoldTimer` 0.0)
        (`/Engine/EditorBlueprintResources/StandardMacros.Gate` false :!label _label_2
          (:`Exit`
            (`KismetSystemLibrary.PrintString` null "Spawn")
            (`self.CloseKillGate`)
            (bind _asurpg_game_mode_2 (cast `URpg_GameMode` (`GameplayStatics.GetGameMode` null)))
            (`URpg_GameMode.RespawnPlayer` _asurpg_game_mode_2 self)))))))

(event `KillTimer`
  (bind _output_get (set `self.KillHoldTimer` (+ (`self.KillHoldTimer`) 0.1)))
  (`KismetSystemLibrary.PrintString` null (`KismetStringLibrary.Conv_DoubleToString` _output_get)))

(event `OpenKillGate`
  (`|ExecutionSequence`
    (:`then_0`
      (goto _label_2 :!via `Open`))
    (:`then_1`
      (goto _label :!via `Open`))))

(event `CloseKillGate`
  (`|ExecutionSequence`
    (:`then_0`
      (goto _label_2 :!via `Close`))
    (:`then_1`
      (goto _label :!via `Close`))))

(fn `UserConstructionScript`)