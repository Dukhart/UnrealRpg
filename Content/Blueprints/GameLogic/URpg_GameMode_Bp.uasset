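; Game mode that handles server-side death and respawning of players through their player controllers.
; RespawnPlayer spawns the controller's CharacterClass at a player start, falling back to the default pawn unless that class derives from it, then possesses the new pawn.
; KillPlayer destroys the controlled pawn.
; Both events update the controller's alive, can-spawn and lockout flags, and respawning also runs the controller's respawn events.
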(event `self.RespawnPlayer`
  (params (InPlayer :type "URpg_PlayerController Object Reference"))
  (bind _characterclass (`URpg_PlayerController.CharacterClass` InPlayer))
  (bind _returnvalue (`KismetMathLibrary.MakeTransform` (.location (`self.GetTransform` (`self.K2_FindPlayerStart` InPlayer))) (.rotation (`self.GetTransform` (`self.K2_FindPlayerStart` InPlayer)))))
  ;[1 1 1] Respawns the player
  (`KismetSystemLibrary.PrintString` "Start Respawn" true true (struct :`G` 0.66 :`B` 1.0 :`A` 1.0) 50.0)
  (`/Engine/EditorBlueprintResources/StandardMacros.IsValid` InPlayer
    (:`Is Valid`
      (`/Engine/EditorBlueprintResources/ActorMacros.Switch Has Authority`
        (:`Authority`
          (if (not (`URpg_PlayerController.bIsAlive` InPlayer))
            (if (`KismetMathLibrary.ClassIsChildOf` _characterclass (`self.DefaultPawnClass`))
              (bind _returnvalue_2 (`|SpawnActorFromClass` _characterclass _returnvalue "AdjustIfPossibleButAlwaysSpawn" "OverrideRootScale" InPlayer))
              (`Controller.Possess` InPlayer _returnvalue_2)
              (else
                (bind _returnvalue_3 (`|SpawnActorFromClass` (`self.DefaultPawnClass`) _returnvalue "AdjustIfPossibleButAlwaysSpawn" "OverrideRootScale" InPlayer))
                (`Controller.Possess` InPlayer _returnvalue_3)))
            (`URpg_PlayerController.RunRespawnEvents` InPlayer)
            (`URpg_PlayerController.SetCanSpawn` InPlayer false)
            (`URpg_PlayerController.SetLockoutDeathNSpawning` InPlayer false)
            (`URpg_PlayerController.SetIsAlive` InPlayer true)))))))

(event `self.KillPlayer`
  (params (InPlayer :type "URpg_PlayerController Object Reference"))
  (bind _returnvalue (`Controller.K2_GetPawn` InPlayer))
  ;[1 1 1] Kills the player
  (`/Engine/EditorBlueprintResources/StandardMacros.IsValid` InPlayer
    (:`Is Valid`
      (`/Engine/EditorBlueprintResources/ActorMacros.Switch Has Authority`
        (:`Authority`
          (if (`URpg_PlayerController.bIsAlive` InPlayer)
            (`/Engine/EditorBlueprintResources/StandardMacros.IsValid` _returnvalue
              (:`Is Valid`
                (`self.K2_DestroyActor` _returnvalue)
                (`URpg_PlayerController.SetIsAlive` InPlayer false)
                (`URpg_PlayerController.SetCanSpawn` InPlayer true)
                (`URpg_PlayerController.SetLockoutDeathNSpawning` InPlayer false))
              (:`Is Not Valid`
                (`KismetSystemLibrary.PrintString` "not valid pawn")))))))
    (:`Is Not Valid`
      (`KismetSystemLibrary.PrintString` "not valid controller"))))

(fn `UserConstructionScript`)